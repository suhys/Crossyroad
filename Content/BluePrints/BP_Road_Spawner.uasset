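; Lane spawner actor that builds a chain of grass, car road and water lanes, starting at the player pawn's location on BeginPlay.
; Each lane spawns at the previous lane's spawn point and receives a reference back to the spawner.
; An integer picks the lane type and is re-rolled randomly after spawning, except after the first grass lane.
; Water only rolls grass or road next, so two water lanes never spawn consecutively.
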(event EventBeginPlay
  (CallFunction|SpawnInitialRoads))

(fn ConstructionScript)

(fn SpawnRoad
  (params (SpawnLocation :type Vector))
  (bind _returnvalue (Math|Random|RandomIntegerinRange 0 2))
  (bind _returnvalue_2 (Math|Random|RandomIntegerinRange 0 2))
  (bind _returnvalue_3 (Math|Random|RandomIntegerinRange 0 1))
  (if (== (Variables|Default|GetNewVar_0) 0)
    (bind _returnvalue_4 (Game|SpawnActorfromClass "/Game/BluePrints/BP_Grass.BP_Grass_C" (Math|Transform|MakeTransform SpawnLocation "0, 0, 0" "1.000000,1.000000,1.000000") "Undefined" 0 0))
    (bind _output_get (Variables|Default|Setnewest_grass _returnvalue_4))
    (Variables|/Game/BluePrints/BP_Grass.BP_Grass_C|SetRoadSpawner _output_get self)
    (bind _output_get_2 (Variables|Default|Setnewest%20road (Transformation|GetWorldLocation (Variables|/Game/BluePrints/BP_Grass.BP_Grass_C|GetG_SpawnPoint (Variables|Default|Getnewest_grass)))))
    (Development|PrintString (Utilities|String|ToString(Vector) _output_get_2))
    (Development|PrintString "new lane reset location")
    (Development|PrintString "Grass Spawned")
    (if (Variables|Default|GetNew%20Var%201)
      (Variables|Default|SetNewVar_0 _returnvalue_2)
      (Development|PrintString (Utilities|String|ToString(Integer) _returnvalue_2)))
    (elif (== (Variables|Default|GetNewVar_0) 1)
      (bind _returnvalue_5 (Game|SpawnActorfromClass "/Game/BluePrints/BP_CarRoad.BP_CarRoad_C" (Math|Transform|MakeTransform SpawnLocation "0, 0, 0" "1.000000,1.000000,1.000000") "Undefined" 0 0))
      (bind _output_get_3 (Variables|Default|Setnewest%20-%20Road _returnvalue_5))
      (Variables|/Game/BluePrints/BP_CarRoad.BP_CarRoad_C|SetRoadSpawner _output_get_3 self)
      (bind _output_get_4 (Variables|Default|Setnewest%20road (Transformation|GetWorldLocation (Variables|/Game/BluePrints/BP_CarRoad.BP_CarRoad_C|GetRoad_Spawn%20Point (Variables|Default|Getnewest%20-%20Road)))))
      (Development|PrintString (Utilities|String|ToString(Vector) _output_get_4))
      (Development|PrintString "new lane reset location")
      (Development|PrintString "Road Spawned")
      (Variables|Default|SetNewVar_0 _returnvalue)
      (Development|PrintString (Utilities|String|ToString(Integer) _returnvalue))
      (else
        (bind _returnvalue_6 (Game|SpawnActorfromClass "/Game/BluePrints/BP_water.BP_water_C" (Math|Transform|MakeTransform SpawnLocation "0, 0, 0" "1.000000,1.000000,1.000000") "Undefined" 0 0))
        (bind _output_get_5 (Variables|Default|Setnewest_Water _returnvalue_6))
        (Variables|/Game/BluePrints/BP_water.BP_water_C|SetRoadSpawner _output_get_5 self)
        (Variables|Default|Setnewest%20road (Transformation|GetWorldLocation (Variables|/Game/BluePrints/BP_water.BP_water_C|GetSpawnPoint (Variables|Default|Getnewest_Water))))
        (Development|PrintString "Water Spawned")
        (Variables|Default|SetNewVar_0 _returnvalue_3)
        (Development|PrintString (Utilities|String|ToString(Integer) _returnvalue_3))))))

(fn SpawnInitialRoads
  (Development|PrintString "Begin for")
  (for _index (range 0 20)
    (Utilities|IsValid (Variables|Default|Getnewest_grass)
      (:Is%20Valid
        (Variables|Default|SetNew%20Var%201 true)
        (Development|PrintString "Hello")
        (Development|PrintString "is valid")
        (CallFunction|SpawnRoadatSpawnPoint))
      (:Is%20Not%20Valid
        (Development|PrintString "is not valid")
        (CallFunction|SpawnRoad (Transformation|GetActorLocation (Game|Player|GetPlayerPawn 0)))))))

(fn SpawnRoadatSpawnPoint
  (bind _newest_road (Variables|Default|Getnewest%20road))
  (Development|PrintString (Utilities|String|ToString(Vector) _newest_road))
  (Development|PrintString "The lane will spawn at:")
  (CallFunction|SpawnRoad _newest_road))
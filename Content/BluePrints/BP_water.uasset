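; Water lane Blueprint that periodically spawns BP_Log_Spawner actors from one of its two ends.
; BeginPlay randomly picks the Start or End side and starts a looping timer with a random interval, both fixed for the actor's lifetime.
; Each tick of that timer has a random chance to spawn, with rotation set by the chosen side.
; When BP_player overlaps TriggerZone, it asks RoadSpawner for a new road and destroys itself.
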(event OnComponentBeginOverlap(TriggerZone)
  (params (OverlappedComponent :type Primitive%20Component%20Object%20Reference) (OtherActor :type Actor%20Object%20Reference) (OtherComp :type Primitive%20Component%20Object%20Reference) (OtherBodyIndex :type Integer) (bFromSweep :type Boolean) (SweepResult :type Hit%20Result%20Structure%20%28by%20ref%29))
  (Utilities|Casting|CastToBP_player OtherActor)
  (Development|PrintString "Water")
  (Default|SpawnRoadatSpawnPoint (Variables|Default|GetRoadSpawner))
  (Actor|DestroyActor))

(event Custom|Spawn%20vehicle
  (if (Math|Random|RandomBool)
    (if (Variables|Default|Getstartingcarlocation)
      (Game|SpawnActorfromClass "/Game/BluePrints/BP_Log_Spawner.BP_Log_Spawner_C" (Math|Transform|MakeTransform (Variables|Default|GetStartlocation) "0,90.000000, 0" "1.000000,1.000000,1.000000") "Undefined" 0 0)
      (else
        (Game|SpawnActorfromClass "/Game/BluePrints/BP_Log_Spawner.BP_Log_Spawner_C" (Math|Transform|MakeTransform (Variables|Default|GetEndlocation) "0,-90.000000, 0" "1.000000,1.000000,1.000000") "Undefined" 0 0)))))

(event Collision|EventActorBeginOverlap
  (params (OtherActor :type Actor%20Object%20Reference)))

(event EventTick
  (params (DeltaSeconds :type Float%20%28single-precision%29)))

(event EventBeginPlay
  (Variables|Default|SetStartlocation (Transformation|GetWorldLocation (Variables|Default|Getstart)))
  (Variables|Default|SetEndlocation (Transformation|GetWorldLocation (Variables|Default|Getend)))
  (Variables|Default|Setstartingcarlocation (Math|Random|RandomBool))
  (Utilities|Time|SetTimerbyEvent (delegate Custom|Spawn%20vehicle) (Math|Random|RandomFloatinRange 1.0 2.0) true))

(fn ConstructionScript)
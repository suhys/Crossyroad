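; BP_Vehicle_Spawner is a moving vehicle hazard that hits the player; despite the name, it spawns nothing itself.
; On BeginPlay a random roll either keeps the defaults or switches the mesh to a red car and overrides the ProjectileMovement initial and max speeds.
; The first collision overlap with BP_player calls Hitbycar on that player, and a DoOnce blocks repeat hits.
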(event OnComponentBeginOverlap(Collision)
  (params (OverlappedComponent :type Primitive%20Component%20Object%20Reference) (OtherActor :type Actor%20Object%20Reference) (OtherComp :type Primitive%20Component%20Object%20Reference) (OtherBodyIndex :type Integer) (bFromSweep :type Boolean) (SweepResult :type Hit%20Result%20Structure%20%28by%20ref%29))
  (bind _asbp_player (Utilities|Casting|CastToBP_player OtherActor))
  (Utilities|FlowControl|DoOnce false
    (:Completed
      (Default|Hitbycar _asbp_player))))

(event EventBeginPlay
  (bind _projectilemovement (Variables|Default|GetProjectileMovement))
  (switch int (Math|Random|RandomIntegerinRange 0 1)
    (:1
      (Variables|/Script/Engine.ProjectileMovementComponent|SetMaxSpeed _projectilemovement 2.5e+02)
      (Variables|/Script/Engine.ProjectileMovementComponent|SetInitialSpeed _projectilemovement 2.5e+02)
      (Components|StaticMesh|SetStaticMesh (Variables|Default|GetStaticMesh) "/Game/crossy_road_meshes/crossy_road_meshes_fbx/redcar_vox.redcar_vox"))))

(fn ConstructionScript)
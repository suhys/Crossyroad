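; BP_RR is a road segment, likely a railroad, that spawns trains and awards score as the player passes.
; On BeginPlay it picks one travel direction and starts a looping timer with a randomized interval; each tick has a random chance to spawn a BP_Train from Start or End.
; A Score overlap updates the player's score once.
; A TriggerZone overlap asks RoadSpawner for another road, then destroys this segment.
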(event OnComponentBeginOverlap(TriggerZone)
  (params (OverlappedComponent :type Primitive%20Component%20Object%20Reference) (OtherActor :type Actor%20Object%20Reference) (OtherComp :type Primitive%20Component%20Object%20Reference) (OtherBodyIndex :type Integer) (bFromSweep :type Boolean) (SweepResult :type Hit%20Result%20Structure%20%28by%20ref%29))
  (Utilities|Casting|CastToBP_player OtherActor)
  (Default|SpawnRoadatSpawnPoint (Variables|Default|GetRoadSpawner))
  (Actor|DestroyActor))

(event OnComponentBeginOverlap(score)
  (params (OverlappedComponent :type Primitive%20Component%20Object%20Reference) (OtherActor :type Actor%20Object%20Reference) (OtherComp :type Primitive%20Component%20Object%20Reference) (OtherBodyIndex :type Integer) (bFromSweep :type Boolean) (SweepResult :type Hit%20Result%20Structure%20%28by%20ref%29))
  (bind _asbp_player (Utilities|Casting|CastToBP_player OtherActor))
  (Utilities|FlowControl|DoOnce false
    (:Completed
      (Default|UpdateScore _asbp_player))))

(event Custom|Spawn%20vehicle
  (if (Math|Random|RandomBool)
    (if (Variables|Default|Getstartingcarlocation)
      (Game|SpawnActorfromClass "/Game/BluePrints/BP_Train.BP_Train_C" (Math|Transform|MakeTransform (Variables|Default|GetStartlocation) "0,90.000000, 0" "1.000000,1.000000,1.000000") "Undefined" 0 0)
      (else
        (Game|SpawnActorfromClass "/Game/BluePrints/BP_Train.BP_Train_C" (Math|Transform|MakeTransform (Variables|Default|GetEndlocation) "0,-90.000000, 0" "1.000000,1.000000,1.000000") "Undefined" 0 0)))))

(event EventBeginPlay
  (Variables|Default|SetStartlocation (Transformation|GetWorldLocation (Variables|Default|Getstart)))
  (Variables|Default|SetEndlocation (Transformation|GetWorldLocation (Variables|Default|Getend)))
  (Variables|Default|Setstartingcarlocation (Math|Random|RandomBool))
  (Utilities|Time|SetTimerbyEvent (delegate Custom|Spawn%20vehicle) (Math|Random|RandomFloatinRange 3.0 4.0) true))

(fn ConstructionScript)